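; Replicator Blueprint that shares Cloud AR Pin names and cloud IDs from the authority to clients as parallel arrays, with name-to-ID lookup.
; Authority adds pins by rebuilding and reassigning each array, since Add does not trigger notify; the names' OnRep refreshes the local ARPlayerController's pin widget.
; SyncCloudARPins forces resync by emptying both arrays, then restoring copies after a short delay.
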(event Custom|SyncCloudARPins
  (bind _idscopy (Variables|Default|GetIDsCopy))
  (bind _namescopy (Variables|Default|GetNamesCopy))
  (Networking|SwitchHasAuthority
    (:Authority
      (Utilities|FlowControl|Sequence
        (:then_0
          ;[1 1 1] Force sync the Name array
          (Utilities|Array|Clear _namescopy)
          (for _array_element (Variables|Default|GetCloudARPinNames)
            (Utilities|Array|Add _namescopy _array_element))
          (Variables|Default|SetCloudARPinNames (Variables|Default|GetEmptyNameArray))
          (Utilities|FlowControl|Delay 0.2)
          (Variables|Default|SetCloudARPinNames _namescopy))
        (:then_1
          ;[1 1 1] Force sync the ID array
          (Utilities|Array|Clear _idscopy)
          (for _array_element_2 (Variables|Default|GetCloudARPinIDs)
            (Utilities|Array|Add _idscopy _array_element_2))
          (Variables|Default|SetCloudARPinIDs (Variables|Default|GetEmptyIDArray))
          (Utilities|FlowControl|Delay 0.2)
          (Variables|Default|SetCloudARPinIDs _idscopy))))))

(fn ConstructionScript)

(fn OnRepCloudARPinNames
  (bind _asarplayer_controller (Utilities|Casting|CastToARPlayerController (Game|GetPlayerController 0)))
  (Utilities|IsValid (Variables|/Game/CloudARPin/Blueprints/ARPlayerController.ARPlayerController_C|GetCloudARPinWidget _asarplayer_controller)
    (:Is%20Valid
      (Default|UpdateCloudARPinIDs (Variables|/Game/CloudARPin/Blueprints/ARPlayerController.ARPlayerController_C|GetCloudARPinWidget _asarplayer_controller) (Variables|Default|GetCloudARPinNames)))))

(fn SetCloudARPinWidget
  (params (Widget :type Cloud%20AR%20Pin%20Widget%20Object%20Reference))
  (Variables|Default|SetCloudARPinWidget Widget))

(fn ReplicateNewCloudARPin
  (params (CloudARPinName :type String) (CloudID :type String))
  (bind _tempnamearray (LocalVariables|GetTempNameArray))
  (bind _tempidarray (LocalVariables|GetTempIDArray))
  (Networking|SwitchHasAuthority
    (:Authority
      (Utilities|FlowControl|Sequence
        (:then_0
          ;[1 1 1] Add the new ARPin Name and trigger the OnRep notify function. We uses a temp array here since Add doesn't trigger notify.
          (for _array_element (Variables|Default|GetCloudARPinNames)
            (Utilities|Array|Add _tempnamearray _array_element))
          (Utilities|Array|Add _tempnamearray CloudARPinName)
          (Variables|Default|SetCloudARPinNames _tempnamearray))
        (:then_1
          ;[1 1 1] Add the CloudARPin CloudID and replicate the value across client.
          (for _array_element_2 (Variables|Default|GetCloudARPinIDs)
            (Utilities|Array|Add _tempidarray _array_element_2))
          (Utilities|Array|Add _tempidarray CloudID)
          (Variables|Default|SetCloudARPinIDs _tempidarray))))))

(fn GetCloudIDfromName
  (params (CloudARPinName :type String))
  (return (Utilities|Array|Get(acopy) (Variables|Default|GetCloudARPinIDs) (Utilities|Array|FindItem (Variables|Default|GetCloudARPinNames) CloudARPinName))))