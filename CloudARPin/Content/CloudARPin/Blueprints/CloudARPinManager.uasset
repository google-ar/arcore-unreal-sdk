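; Manager actor for a multiplayer shared-AR session: the server hosts a Cloud AR Pin, clients resolve it, then players tap to place objects.
; A validated state machine drives Tick and touch handling and updates snackbar messages.
; The CloudID on MultiplayerARSceneRoot links host to clients, and placements reach the server as transforms relative to that root.
; Non-AR platforms simulate hosting, resolving and placement with a plane and random outcomes.
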(event EventBeginPlay
  (bind _simulatedplane (Variables|Default|GetSimulatedPlane))
  (Utilities|IsARSupportedPlatform
    (:true
      (Rendering|SetActorHiddenInGame _simulatedplane true))
    (:false
      (Rendering|SetActorHiddenInGame _simulatedplane false)))
  ;[1 1 1] Wait the ARPlayerController to create the UIWidget and get the reference
  (Utilities|FlowControl|Delay 0.2)
  (bind _asarplayer_controller (Utilities|Casting|CastToARPlayerController (Game|GetPlayerController 0)))
  (Variables|Default|SetCloudARPinWidget (Variables|/Game/CloudARPin/Blueprints/ARPlayerController.ARPlayerController_C|GetCloudARPinWidget _asarplayer_controller))
  (Networking|SwitchHasAuthority
    (:Authority
      _)
    (:Remote
      ;[1 1 1] Find and set the ARSceneRoot actor spawned by the server
      (bind _outactors (Actor|GetAllActorsOfClass "/Game/CloudARPin/Blueprints/MultiplayerARSceneRoot.MultiplayerARSceneRoot_C"))
      (Variables|Default|SetARSceneRoot (Utilities|Array|Get(acopy) _outactors))))
  ;[1 1 1] Set the initial game state for server and client
  (bind _asargame_instance (Utilities|Casting|CastToARGameInstance (Game|GetGameInstance)))
  (Variables|Default|SetARGameInstance _asargame_instance)
  (if (Ability|HasAuthority)
    (Utilities|TransitiontoGameState "NewEnumerator4")
    (else
      (Utilities|TransitiontoGameState "NewEnumerator1"))))

(event EventTick
  (params (DeltaSeconds :type Float%20%28single-precision%29))
  ;[1 1 1] Tick the Actor based on the current game state
  (switch Utilities|FlowControl|Switch|SwitchonCloudARPinGameState (Variables|Default|GetCurrentGameState)
    (:NewEnumerator4
      (Utilities|CheckARPlaneDetected))
    (:NewEnumerator1
      (Utilities|CheckCloudIDSynced))
    (:NewEnumerator3
      (Utilities|ResolveCloudARPinRoot))))

(event Input|TouchEvents|InputTouch
  (params (Location :type Vector) (FingerIndex :type ETouchIndex%20Enum))
  (:Pressed
    ;[1 1 1] Handle touch event based on the current game state
    (switch Utilities|FlowControl|Switch|SwitchonCloudARPinGameState (Variables|Default|GetCurrentGameState)
      (:NewEnumerator0
        (Utilities|HostCloudARPinRoot FingerIndex))
      (:NewEnumerator5
        (Utilities|PlaceGameActor FingerIndex)))))

(fn ConstructionScript)

(fn GetCloudARPinError
  (params (CloudPin :type Cloud%20AR%20Pin%20Object%20Reference) (TaskResult :type EARPinCloudTaskResult%20Enum :default "Success"))
  (if (Utilities|IsValid CloudPin)
    (return (Utilities|String|EnumtoString (Class|CloudARPin|GetARPinCloudState CloudPin)))
    (else
      (return (Utilities|String|EnumtoString TaskResult)))))

(fn GetRelativeTransfromtoARSceneRoot
  (params (ChildActorWorldTransform :type Transform))
  (bind _arsceneroot (Variables|Default|GetARSceneRoot))
  (bind _cloudarpinroot (Variables|/Game/CloudARPin/Blueprints/MultiplayerARSceneRoot.MultiplayerARSceneRoot_C|GetCloudARPinRoot _arsceneroot))
  (bind _returnvalue (Transformation|GetWorldTransform _cloudarpinroot))
  (return (Math|Transform|MakeTransform (Math|Transform|InverseTransformLocation _returnvalue (.location ChildActorWorldTransform)) (Math|Transform|InverseTransformRotation _returnvalue (.rotation ChildActorWorldTransform)))))