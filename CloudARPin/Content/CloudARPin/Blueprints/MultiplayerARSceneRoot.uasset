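; MultiplayerARSceneRoot is an actor that anchors a shared AR scene to a Cloud AR Pin.
; On the authority it copies the room ID from the AR game instance at BeginPlay and accepts cloud ID updates through SetCloudID.
; AttachToCloudARPin stores the pin locally, and each Tick moves CloudARPinRoot to the pin's transform while the pin is valid and tracking.
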(event EventBeginPlay
  (Networking|SwitchHasAuthority
    (:Authority
      (bind _asargame_instance (Utilities|Casting|CastToARGameInstance (Game|GetGameInstance)))
      (Variables|Default|SetRoomID (Variables|/Game/CloudARPin/Blueprints/ARGameInstance.ARGameInstance_C|GetRoomID _asargame_instance)))))

(event EventTick
  (params (DeltaSeconds :type Float%20%28single-precision%29))
  (bind _cloudarpin (Variables|Default|GetCloudARPin))
  (if (Utilities|IsValid (Variables|Default|GetCloudARPin))
    (if (Utilities|Enum|Equal(Enum) (Class|ARPin|GetTrackingState _cloudarpin) "Tracking")
      (Transformation|SetWorldTransform (Variables|Default|GetCloudARPinRoot) (Class|ARPin|GetLocaltoWorldTransform _cloudarpin) false false))))

(fn ConstructionScript)

(fn SetCloudID
  (params (CloudID :type String))
  (Networking|SwitchHasAuthority
    (:Authority
      (Variables|Default|SetCloudID CloudID))))

(fn AttachtoCloudARPin
  (params (CloudARPin :type Cloud%20AR%20Pin%20Object%20Reference))
  (Variables|Default|SetCloudARPin CloudARPin))