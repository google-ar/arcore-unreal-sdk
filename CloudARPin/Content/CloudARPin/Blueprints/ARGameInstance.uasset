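; Game instance for CloudARPin that hosts and joins LAN multiplayer sessions, opening the CloudARPin level as a listen server.
; Joining with a blank IP takes the first session found; a typed IP uses the console open command, reporting failure if MainMenu is still loaded after a delay.
; The IP check range-tests four-part dotted addresses but accepts any other format.
; Failures appear in a single reused ErrorDialog widget.
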(event Custom|StartSession
  (|Session (Game|GetPlayerController 0) 4 true
    (:OnSuccess
      (Game|OpenLevel(byName) "CloudARPin" true "?Listen"))
    (:OnFailure
      (CallFunction|ShowDialog "Failed to create session."))))

(event Custom|Join%20Session
  (params (ServerIPAddress :type String))
  (bind _returnvalue (Game|GetPlayerController 0))
  (if (Utilities|Enum|Equal(Enum) ServerIPAddress "")
    ;[1 1 1] Search for hosted session and join the first one if the IP input box is blank.
    (bind _results (|FindSessions _returnvalue 5 true)
      (:OnSuccess
        (Utilities|SessionFound _results
          (:then
            (|JoinSession _returnvalue (Utilities|Array|Get(acopy) _results)
              (:OnFailure
                (CallFunction|ShowDialog "Failed to join the session."))))
          (:else
            (CallFunction|ShowDialog "No game session found"))))
      (:OnFailure
        (CallFunction|ShowDialog "Find session failed")))
    (else
      ;[1 1 1] Join the session using the input IP address
      (bind _isvalid (CallFunction|IsValidIPAddress ServerIPAddress))
      (if _isvalid
        (Development|ExecuteConsoleCommand (Utilities|String|Append "open " ServerIPAddress) 0)
        (Utilities|FlowControl|Delay 5.0)
        (bind _returnvalue_2 (Game|GetCurrentLevelName true))
        (if (Utilities|Enum|Equal(Enum) _returnvalue_2 "MainMenu")
          (CallFunction|ShowDialog (Utilities|Text|ToText(String) (Utilities|String|Append "Failed to join the session hosted at IP: " ServerIPAddress))))
        (else
          (CallFunction|ShowDialog "Invalid IP Address"))))))

(fn ShowDialog
  (params (Message :type Text))
  (Utilities|IsValid (Variables|Default|GetErrorDialog)
    (:Is%20Valid
      (Widget|SetVisibility (Variables|Default|GetErrorDialog) "Visible"))
    (:Is%20Not%20Valid
      (bind _returnvalue (UserInterface|CreateWidget "/Game/CloudARPin/Blueprints/ErrorDialog.ErrorDialog_C"))
      (Variables|Default|SetErrorDialog _returnvalue)
      (UserInterface|Viewport|AddtoViewport (Variables|Default|GetErrorDialog) 0)))
  (Variables|/Game/CloudARPin/Blueprints/ErrorDialog.ErrorDialog_C|SetMessage (Variables|Default|GetErrorDialog) Message))

(fn IsValidIPAddress
  (params (SourceString :type String))
  (bind _returnvalue (Utilities|String|ParseIntoArray SourceString "."))
  (if (== (Utilities|Array|Length _returnvalue) 4)
    (for _array_element _returnvalue
      (if (not (Math|Integer|InRange(Integer) (Math|Conversions|ToInteger(Byte) _array_element) 0 255))
        (return false)))
    (return true)
    (else
      (return (>= (Utilities|Array|Length (Utilities|String|ParseIntoArray SourceString ":")) 0)))))