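; Player controller for a multiplayer Cloud AR Pin (GoogleARCore) game that runs the local AR session and adds the HUD widget.
; Tick finds the replicated scene root, reports session failures on the snackbar, and toggles the screensaver and scene/plane visibility when tracking quality changes.
; A server event spawns game actors attached to the scene root by relative transform.
; Android Back destroys the online session and returns to the main menu.
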(event Custom|ServerAddGameActor
  (params (RelativeTransform :type Transform))
  ;[1 1 1] On server, spawn the game actor and attach it to ARSceneRoot actor using the relative transform passed in
  (bind _returnvalue (Game|SpawnActorfromClass "/Game/CloudARPin/Blueprints/GameActor.GameActor_C" (Math|Transform|MakeTransform "0, 0, 0" "0, 0, 0" "1,1,1") "Undefined" 0 0))
  (Transformation|AttachActorToActor _returnvalue (Variables|Default|GetARSceneRoot) "None" "KeepRelative" "KeepRelative" "KeepRelative" true)
  (Transformation|SetActorRelativeTransform _returnvalue RelativeTransform false false))

(event EventBeginPlay
  ;[1 1 1] Create UIWidget for local player
  (if (Pawn|IsLocalPlayerController)
    (bind _returnvalue (UserInterface|CreateWidget "/Game/CloudARPin/Blueprints/CloudARPinWidget.CloudARPinWidget_C" self))
    (bind _output_get (Variables|Default|SetCloudARPinWidget _returnvalue))
    (UserInterface|Viewport|AddtoViewport _output_get 0)
    ;[1 1 1] Enable GoogleARCore Services and start ARSession
    (Utilities|IsARSupportedPlatform
      (:true
        (Class|GoogleARCoreServicesFunctionLibrary|ConfigGoogleARCoreServices (Utilities|Struct|MakeGoogleARCoreServicesConfig "Enabled"))
        (Class|ARBlueprintLibrary|StartARSession "/Game/CloudARPin/Blueprints/CloudARPinSessionConfig.CloudARPinSessionConfig")
        (CallFunction|UpdateScreensaver)))))

(event EventTick
  (params (DeltaSeconds :type Float%20%28single-precision%29))
  (bind _returnvalue (Class|ARBlueprintLibrary|GetTrackingQuality))
  (bind _returnvalue_2 (Class|ARBlueprintLibrary|GetARSessionStatus))
  (Utilities|FlowControl|Sequence
    (:then_0
      ;[1 1 1] Get the ARSceneRoot Actor reference when it is spawned by the server
      (Utilities|IsValid (Variables|Default|GetARSceneRoot)
        (:Is%20Not%20Valid
          (bind _outactors (Actor|GetAllActorsOfClass "/Game/CloudARPin/Blueprints/MultiplayerARSceneRoot.MultiplayerARSceneRoot_C"))
          (if (> (Utilities|Array|Length _outactors) 0)
            (Variables|Default|SetARSceneRoot (Utilities|Array|Get(acopy) _outactors))))))
    (:then_1
      ;[1 1 1] Show error when ARSession failed to start
      (switch Utilities|FlowControl|Switch|SwitchonEARSessionStatus (.status _returnvalue_2)
        (:Running
          (Utilities|FlowControl|Sequence
            (:then_0
              (if (!= (Variables|Default|GetPreviousTrackingQuality) _returnvalue)
                (CallFunction|UpdateScreensaver)
                (CallFunction|UpdateSceneActorVisibility)))
            (:then_1
              (Variables|Default|SetPreviousTrackingQuality _returnvalue))))
        (:NotSupported
          (Default|SetSnackbarOutput (Variables|Default|GetCloudARPinWidget) (Utilities|Text|ToText(String) (Utilities|Select :Index (.status _returnvalue_2) :NotStarted "" :Running "" :NotSupported "AR session failed to start becuase the device is not supported" :FatalError "AR session has unknown error." :PermissionNotGranted "Camera unavailable. Please restart the app." :UnsupportedConfiguration "" :Other "")) :!label _label))
        (:FatalError
          (goto _label))
        (:PermissionNotGranted
          (goto _label))))))

(event EventEndPlay
  (params (EndPlayReason :type EEndPlayReason%20Enum :default "Destroyed"))
  ;[1 1 1] Stop ARSession
  (if (Pawn|IsLocalPlayerController)
    (Class|ARBlueprintLibrary|StopARSession)))

(event Input|KeyboardEvents|AndroidBack
  (params (Key :type Key%20Structure))
  (:Pressed
    ;[1 1 1] Return to main menu when Android back button is pressed
    (if (Pawn|IsLocalPlayerController)
      (|DestroySession self
        (:OnSuccess
          _)
        (:OnFailure
          _))
      (Game|OpenLevel(byName) "MainMenu"))))

(fn ConstructionScript)

(fn UpdateScreensaver
  (switch Utilities|FlowControl|Switch|SwitchonEARTrackingQuality (Class|ARBlueprintLibrary|GetTrackingQuality)
    (:NotTracking
      (if (not (Variables|Default|GetScreenSaverEnabled))
        (Class|KismetSystemLibrary|ControlScreensaver true)
        (Variables|Default|SetScreenSaverEnabled true)))
    (:OrientationAndPosition
      (if (Variables|Default|GetScreenSaverEnabled)
        (Class|KismetSystemLibrary|ControlScreensaver false)
        (Variables|Default|SetScreenSaverEnabled false)))))

(fn UpdateSceneActorVisibility
  (bind _returnvalue (Class|ARBlueprintLibrary|GetTrackingQuality))
  (bind _returnvalue_2 (Utilities|Select :Index _returnvalue :NotTracking false :OrientationOnly false :OrientationAndPosition true))
  (Rendering|SetVisibility (Variables|/Game/CloudARPin/Blueprints/MultiplayerARSceneRoot.MultiplayerARSceneRoot_C|GetCloudARPinRoot (Variables|Default|GetARSceneRoot)) _returnvalue_2 true)
  (bind _outactors (Actor|GetAllActorsOfClass "/Script/CloudARPinSample.ARPlaneRenderer"))
  (Rendering|SetVisibility (Variables|/Script/Engine.Actor|GetRootComponent (Utilities|Array|Get(acopy) _outactors)) _returnvalue_2 true))